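; BP_D_TestLeftDown is a test destructible that breaks when the player is in the required stance and position.
; CheckDestructuble requires player Stance 1 (apparently left-down) and overlap with the AttackPoseCheck volume, without checking for an actual attack.
; It then, once only, removes all anchors from its geometry collection and spawns BP_MasterfieldTest at that transform.
; Tick and overlap events are empty, so the check depends on CheckDestructuble being called.
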(event `self.ReceiveBeginPlay`)

(event `self.ReceiveTick`
  (params (DeltaSeconds :type "Float (single-precision)"))
  ;[1 1 1] EVENT Tick Yerine nerede çalışabilir?
)

(event `/Game/Exol/Assets/Destructubles/BPI_Destructble.checkDestructuble`
  (bind _fracturetest_geometrycollection (`self.FractureTest_GeometryCollection`))
  (`KismetSystemLibrary.PrintString` "geldikkk")
  (bind _asbp_player (cast `/Game/Exol/Blueprint/Bp_Player` (`GameplayStatics.GetPlayerPawn` 0)))
  ;[1 0.1439 0] LeftDownMu Stance? (attack gerçekleşti mi sorgusu yok??)
  (if (== (`/Game/Exol/Blueprint/Bp_Player.Stance` _asbp_player) 1)
    ;[1 1 1] Player kesmek için doğru yönde mi?
    (for _array_element (`PrimitiveComponent.GetOverlappingActors` (`self.AttackPoseCheck`) null)
      (if (== _asbp_player _array_element)
        (`/Engine/EditorBlueprintResources/StandardMacros.DoOnce` false
          (:`Completed`
            (`GeometryCollectionComponent.RemoveAllAnchors` _fracturetest_geometrycollection)
            (`|SpawnActorFromClass` "/Game/Exol/Assets/Destructubles/BP_MasterfieldTest.BP_MasterfieldTest_C" (`SceneComponent.K2_GetComponentToWorld` _fracturetest_geometrycollection) "Undefined" "OverrideRootScale" null null)))))))

(fn `UserConstructionScript`)