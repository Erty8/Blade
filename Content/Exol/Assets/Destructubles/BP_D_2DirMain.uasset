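; BP_D_2DirMain is a destructible wall that breaks when CheckDestructable is called while the player's stance is either of two set directions.
; A correct stance fires a DoOnce that makes the WallGC geometry collection dynamic, removes its anchors, spawns a BP_MasterfieldTest at the impact point and plays a break sound.
; A wrong stance plays a fail sound and briefly puffs misdirection dust.
; Overlap-side checks and collapse cleanup are present but disconnected.
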(event `/Game/Exol/Blueprint/Interfaces/BPI_Destructable.checkDestructable`
  (params (ImpactPoint :type "Vector Structure"))
  (bind _wrongdirdust (`self.WrongDirDust`))
  (bind _wallgc (`self.wallGC`))
  ;[1 1 1] Check Stance
  (bind _asbp_player (cast `/Game/Exol/Blueprint/Bp_Player` (`GameplayStatics.GetPlayerPawn` 0) :!label _label)
    (:`then`
      (bind _stance (`/Game/Exol/Blueprint/Bp_Player.Stance` _asbp_player))
      (if (or (== _stance (`self.Direction1`)) (== _stance (`self.Direction2`)))
        (`/Engine/EditorBlueprintResources/StandardMacros.DoOnce` false
          (:`Completed`
            (`KismetSystemLibrary.PrintString` "success")
            (cast `/Game/Exol/Blueprint/Bp_Player` (`GameplayStatics.GetPlayerPawn` 0))
            (set `GeometryCollectionComponent.ObjectType` "Chaos_Object_Dynamic" (`self.wallGC`))
            ;[1 1 1] To keep in position until the attack from correct stance is executed
            (`KismetSystemLibrary.Delay` 0.05)
            (`GeometryCollectionComponent.RemoveAllAnchors` _wallgc)
            (`KismetSystemLibrary.PrintString` "Anchor removed")
            (bind _returnvalue (`|SpawnActorFromClass` "/Game/Exol/Assets/Destructubles/BP_MasterfieldTest.BP_MasterfieldTest_C" (`KismetMathLibrary.Conv_VectorToTransform` ImpactPoint) "AlwaysSpawn" "MultiplyWithRoot" null null))
            (`GameplayStatics.PlaySoundAtLocation` "/Game/Exol/Assets/Sound/SFX/WoodLogDestroy.WoodLogDestroy" (`SceneComponent.K2_GetComponentLocation` _wallgc) (struct) 0.5 1.0 0.1 null null null null)
            (`KismetSystemLibrary.Delay` 0.1)))
        (else
          (`GameplayStatics.PlaySoundAtLocation` "/Game/Exol/Assets/Sound/SFX/WoodLogFail.WoodLogFail" (0.0 0.0 0.0) (struct) 1.0 1.0 0.0 null null null null)
          ;[1 1 1] Misdirection Dust
          (`ActorComponent.Activate` _wrongdirdust false)
          (`ActorComponent.Activate` (`self.WrongDirDust1`) false)
          (`KismetSystemLibrary.Delay` 0.2)
          (`ActorComponent.Deactivate` _wrongdirdust)
          (`ActorComponent.Deactivate` (`self.WrongDirDust1`))
          (`/Engine/EditorBlueprintResources/StandardMacros.DoOnce` false :!via `Reset`
            (:`Completed`
              (goto _label))))))
    (:`CastFailed`
      (`KismetSystemLibrary.PrintString` "CAST FAILED" true true (struct :`R` 1.0 :`B` 0.717875 :`A` 1.0)))))

(fn `UserConstructionScript`)