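; BP_D_AnyAttack is a destructible Geometry Collection wall that breaks when its CheckDestructable event is called with an impact point.
; The event fires only once, removing all anchors from WallGC and spawning a BP_MasterfieldTest field actor at the impact.
; It plays a wood destruction sound and briefly activates two dust effects, destroying the field actor after a short delay.
; AnyDamage is empty, and debug prints remain.
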(event `/Game/Exol/Blueprint/Interfaces/BPI_Destructable.checkDestructable`
  (params (ImpactPoint :type "Vector Structure"))
  (bind _wrongdirdust (`self.WrongDirDust`))
  (bind _wallgc (`self.wallGC`))
  (`KismetSystemLibrary.PrintString` "check destructable called")
  (`KismetSystemLibrary.PrintString` "before do once")
  (`/Engine/EditorBlueprintResources/StandardMacros.DoOnce` false
    (:`Completed`
      (`KismetSystemLibrary.PrintString` "do ONCE")
      (`GeometryCollectionComponent.RemoveAllAnchors` _wallgc)
      (bind _returnvalue (`|SpawnActorFromClass` "/Game/Exol/Assets/Destructubles/BP_MasterfieldTest.BP_MasterfieldTest_C" (`KismetMathLibrary.Conv_VectorToTransform` ImpactPoint) "Undefined" "MultiplyWithRoot" null null))
      (`GameplayStatics.PlaySoundAtLocation` "/Game/Exol/Assets/Sound/SFX/WoodCreateDestroy.WoodCreateDestroy" (`SceneComponent.K2_GetComponentLocation` _wallgc) (struct) 0.1 1.0 0.0 null null null null)
      (`ActorComponent.Activate` _wrongdirdust false)
      (`ActorComponent.Activate` (`self.WrongDirDust1`) false)
      (`KismetSystemLibrary.Delay` 0.2)
      (`self.K2_DestroyActor` _returnvalue)
      (`ActorComponent.Deactivate` _wrongdirdust)
      (`ActorComponent.Deactivate` (`self.WrongDirDust1`)))))

(event `self.ReceiveAnyDamage`
  (params (Damage :type "Float (single-precision)") (DamageType :type "DamageType Object Reference") (InstigatedBy :type "Controller Object Reference") (DamageCauser :type "Actor Object Reference")))

(fn `UserConstructionScript`)