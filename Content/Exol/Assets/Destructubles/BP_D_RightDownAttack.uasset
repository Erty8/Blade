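; Destructible Geometry Collection wall that breaks only for the player's right-down attack stance.
; CheckDestructuble requires Bp_Player stance 4 and overlap with AttackPoseCheck, without verifying that an attack occurred.
; On success it runs once, removing WallGC anchors, spawning a BP_MasterfieldTest field actor and playing a wood-break sound.
; A wrong stance briefly pulses two misdirection dust effects using delays.
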(event `self.ReceiveTick`
  (params (DeltaSeconds :type "Float (single-precision)"))
  ;[1 1 1] EVENT Tick Yerine nerede çalışabilir?
)

(event `/Game/Exol/Assets/Destructubles/BPI_Destructble.checkDestructuble`
  (bind _wrongdirdust (`self.WrongDirDust`))
  (bind _wallgc (`self.wallGC`))
  (`KismetSystemLibrary.PrintString` "geldikkk")
  (bind _asbp_player (cast `/Game/Exol/Blueprint/Bp_Player` (`GameplayStatics.GetPlayerPawn` 0)))
  ;[1 0.1439 0] LeftDownMu Stance? (attack gerçekleşti mi sorgusu yok??)
  (if (== (`/Game/Exol/Blueprint/Bp_Player.Stance` _asbp_player) 4)
    ;[1 1 1] Player kesmek için doğru yönde mi?
    (for _array_element (`PrimitiveComponent.GetOverlappingActors` (`self.AttackPoseCheck`) null)
      (if (== _asbp_player _array_element)
        (`/Engine/EditorBlueprintResources/StandardMacros.DoOnce` false
          (:`Completed`
            (`GeometryCollectionComponent.RemoveAllAnchors` _wallgc)
            (`|SpawnActorFromClass` "/Game/Exol/Assets/Destructubles/BP_MasterfieldTest.BP_MasterfieldTest_C" (`SceneComponent.K2_GetComponentToWorld` _wallgc) "Undefined" "OverrideRootScale" null null)
            (`GameplayStatics.PlaySoundAtLocation` "/Game/Exol/Assets/Sound/SFX/WoodCreateDestroy.WoodCreateDestroy" (`SceneComponent.K2_GetComponentLocation` _wallgc) (struct) 1.0 1.0 0.0 null null null null)))))
    (else
      (`KismetSystemLibrary.Delay` 0.2)
      ;[1 1 1] Misdirection Dust
      (`ActorComponent.Activate` _wrongdirdust false)
      (`ActorComponent.Activate` (`self.WrongDirDust1`) false)
      (`KismetSystemLibrary.Delay` 0.2)
      (`ActorComponent.Deactivate` _wrongdirdust)
      (`ActorComponent.Deactivate` (`self.WrongDirDust1`)))))

(fn `UserConstructionScript`)