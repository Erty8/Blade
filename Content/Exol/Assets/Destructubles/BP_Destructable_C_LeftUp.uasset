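; BP_Destructable_C_LeftUp is a destructible wall that breaks only when the player's stance matches one of two accepted directions.
; CheckDestructable reads the Bp_Player stance and, on a match, removes all anchors from the WallGC geometry collection once and plays a wood destruction sound.
; WallGC collision is disabled after a delay.
; A wrong stance briefly pulses two dust effects as misdirection feedback.
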(event `self.ReceiveAnyDamage`
  (params (Damage :type "Float (single-precision)") (DamageType :type "DamageType Object Reference") (InstigatedBy :type "Controller Object Reference") (DamageCauser :type "Actor Object Reference")))

(event `/Game/Exol/Blueprint/Interfaces/BPI_Destructable.checkDestructable`
  (bind _wrongdirdust (`self.WrongDirDust`))
  (bind _wallgc (`self.wallGC`))
  (`KismetSystemLibrary.PrintString` "mesah" true true (struct :`R` 0.233694 :`G` 1.0 :`A` 1.0))
  ;[1 1 1] Check Stance
  (bind _asbp_player (cast `/Game/Exol/Blueprint/Bp_Player` (`GameplayStatics.GetPlayerPawn` 0)))
  (bind _stance (`/Game/Exol/Blueprint/Bp_Player.Stance` _asbp_player))
  (if (or (== _stance (`self.Direction1`)) (== _stance (`self.Direction2`)))
    (`/Engine/EditorBlueprintResources/StandardMacros.DoOnce` false
      (:`Completed`
        (cast `/Game/Exol/Blueprint/Bp_Player` (`GameplayStatics.GetPlayerPawn` 0))
        ;[1 1 1] Execute Destroy
        (`GeometryCollectionComponent.RemoveAllAnchors` _wallgc)
        (`GameplayStatics.PlaySoundAtLocation` "/Game/Exol/Assets/Sound/SFX/WoodCreateDestroy.WoodCreateDestroy" (`SceneComponent.K2_GetComponentLocation` _wallgc) (struct) 1.0 1.0 0.0 null null null null)
        (`KismetSystemLibrary.Delay` 4.0)
        (`KismetSystemLibrary.PrintString` "SET COLLISON WALLGC" true true (struct :`R` 1.0 :`G` 0.111651 :`B` 0.796477 :`A` 1.0))
        (`PrimitiveComponent.SetCollisionEnabled` (`self.wallGC`) "NoCollision")))
    (else
      (`KismetSystemLibrary.Delay` 0.2)
      ;[1 1 1] Misdirection Dust
      (`ActorComponent.Activate` _wrongdirdust false)
      (`ActorComponent.Activate` (`self.WrongDirDust1`) false)
      (`KismetSystemLibrary.Delay` 0.2)
      (`ActorComponent.Deactivate` _wrongdirdust)
      (`ActorComponent.Deactivate` (`self.WrongDirDust1`)))))

(fn `UserConstructionScript`)