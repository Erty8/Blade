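; Sword-fighting enemy character with directional attacks that the player can parry by matching stance.
; Each attack plays a stance montage, opens a parry window and shows a hit-indicator widget, then picks the next random stance.
; Incoming damage is sized by player stance and resolves as block with counterattack, parry, or a hit with hit-stop.
; Also drives health bar, spline patrol and death, reporting a saved ID to the game mode.
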(event `self.ReceiveBeginPlay`
  (`self.Attack Pos`)
  (`self.EnemyHealthBarGenerator`))

(event `self.ReceiveTick`
  (params (DeltaSeconds :type "Float (single-precision)"))
  (`self.Face Player`))

(event `self.Sphere.OnComponentBeginOverlap`
  (params (OverlappedComponent :type "PrimitiveComponent Object Reference") (OtherActor :type "Actor Object Reference") (OtherComp :type "PrimitiveComponent Object Reference") (OtherBodyIndex :type Integer) (bFromSweep :type Boolean) (SweepResult :type "HitResult Structure (by ref)"))
  (cast `/Game/Exol/Blueprint/Bp_Player` OtherActor)
  (set `self.playerInrange` true))

(event `self.Sphere.OnComponentEndOverlap`
  (params (OverlappedComponent :type "PrimitiveComponent Object Reference") (OtherActor :type "Actor Object Reference") (OtherComp :type "PrimitiveComponent Object Reference") (OtherBodyIndex :type Integer))
  (cast `/Game/Exol/Blueprint/Bp_Player` OtherActor)
  (set `self.playerInrange` false))

(event `self.ChangeState`
  ;[1 1 1] Destroys Actor If Save Data Calls it 'DEAD'
  (`self.K2_DestroyActor`))

(event `self.ReceiveAnyDamage`
  (params (Damage :type "Float (single-precision)") (DamageType :type "DamageType Object Reference") (InstigatedBy :type "Controller Object Reference") (DamageCauser :type "Actor Object Reference"))
  (`self.PAttackType`)
  (bind _blocked (`self.CheckDamage`))
  ;[0 1 0.2669] EnemyBlockParticle
  (if _blocked
    (`self.ParticleSpawn` :!via `EnemyBlock`)))

(event `self.ReceiveHit`
  (params (MyComp :type "PrimitiveComponent Object Reference") (Other :type "Actor Object Reference") (OtherComp :type "PrimitiveComponent Object Reference") (bSelfMoved :type Boolean) (HitLocation :type "Vector Structure") (HitNormal :type "Vector Structure") (NormalImpulse :type "Vector Structure") (Hit :type "HitResult Structure (by ref)")))

(event `Attack`
  ;[1 1 1] Attacking
  (set `self.Busy` true)
  (`self.Parriable`)
  (`self.PositionMacro`
    (:`NewParam`
      (`self.Attack Pos`))))

(event `OnComponentHit_Event`
  (params (HitComponent :type "PrimitiveComponent Object Reference") (OtherActor :type "Actor Object Reference") (OtherComp :type "PrimitiveComponent Object Reference") (NormalImpulse :type "Vector Structure") (Hit :type "HitResult Structure (by ref)")))

(event `Defend`
  (if (>= (`self.Stamina`) 1.0)
    (set `self.Busy` true)
    (set `self.Blocking` true)
    (`|PlayMontage` (`self.Mesh`) "/Game/Exol/Assets/Enemies/02/animations/BlockM.BlockM"
      (:`then`
        (`MovementComponent.StopMovementImmediately` (`self.CharacterMovement`)))
      (:`OnCompleted`
        (set `self.Blocking` false)
        (set `self.Busy` false)))))

(event `Walk`
  (set `CharacterMovementComponent.MaxWalkSpeed` 150.0 (`self.CharacterMovement`)))

(event `Run`
  (set `CharacterMovementComponent.MaxWalkSpeed` 400.0 (`self.CharacterMovement`)))

(event `CounterAttack`
  (`KismetSystemLibrary.Delay` 0.0)
  (set `self.Blocking` false)
  (`self.Attack`))

(event `Parriable`
  ;[0.2812 0.2812 0.2812] Parry
  (`self.Next Pos To Get Parried` (`self.AtkStance`) true)
  (set `self.CanParried` true)
  (`KismetSystemLibrary.Delay` 0.0))

(event `CheckParry`
  ;[0.2812 0.2812 0.2812] Parry
  (bind _success (`self.IsParrySuccess`))
  (if _success
    (set `self.CanParried` false)
    (`|ExecutionSequence`
      (:`then_0`
        (`self.ParticleSpawn` :!via `Parry`))
      (:`then_1`
        (`|PlayMontage` (`self.Mesh`) "/Game/Exol/Assets/Enemies/02/animations/GetParried.GetParried" 0.8
          (:`then`
            (`GameplayStatics.PlaySoundAtLocation` "/Game/Exol/Assets/Sound/SFX/Sword/warfare_swords_x_2_hit_scrape_003.warfare_swords_x_2_hit_scrape_003" (0.0 0.0 0.0) (struct) 1.0 1.0 0.0 null null null null))
          (:`OnCompleted`
            (set `self.Busy` false)))))
    (else
      (bind _alive (`self.TakeDamage`))
      (if _alive
        (`|PlayMontage` (`self.Mesh`) "/Game/Exol/Assets/Enemies/02/animations/AI_TakeDamage.AI_TakeDamage"
          (:`then`
            (set `self.Busy` true)
            (`self.ParticleSpawn`
              (:`NewParam2`
                (if (`|EnumEquality` (`self.Type`) "NewEnumerator1")
                  (bind _aslevel_2_enemy (cast `/Game/Exol/Blueprint/Enemies/Level2_Enemy` self))
                  (`/Game/Exol/Blueprint/Enemies/Level2_Enemy.Block` _aslevel_2_enemy)))))
          (:`OnCompleted`
            (set `self.Busy` false))
          (:`OnNotifyBegin`
            (if (`self.PSpecial`)
              (goto _label :!via `Special`)
              (else
                (`self.HitStop` :!label _label)))))
        (else
          (set `self.Busy` true)
          (`self.ParticleSpawn`))))))

(event `self.CapsuleComponent.OnComponentBeginOverlap`
  (params (OverlappedComponent :type "PrimitiveComponent Object Reference") (OtherActor :type "Actor Object Reference") (OtherComp :type "PrimitiveComponent Object Reference") (OtherBodyIndex :type Integer) (bFromSweep :type Boolean) (SweepResult :type "HitResult Structure (by ref)"))
  ;[1 1 1] New combat system (collision based)
)

(fn `Attack Pos`
  (returns (Position :type "/Game/Exol/AI/BP_enum_direction Enum"))
  (bind _output_get (set `self.AtkStance` (`KismetArrayLibrary.Array_Random` (`self.MoveList`))))
  (`self.Next Pos To Get Parried` _output_get)
  (return _output_get))

(fn `BloodTrail`)

(fn `CheckDamage`
  (returns (Blocked :type Boolean))
  (if (`self.Blocking`)
    (`GameplayStatics.PlaySoundAtLocation` "/Game/Exol/Assets/Sound/SFX/Sword/warfare_swords_x_2_hit_002.warfare_swords_x_2_hit_002" (`self.K2_GetActorLocation`) (struct) 1.0 1.0 0.0 null null null null)
    (set `self.Stamina` (`KismetMathLibrary.Conv_IntToDouble` (- (`self.Stamina`) 1)))
    (`self.CounterAttack`)
    (return true)
    (else
      (`self.CheckParry`)
      (return false))))

(fn `DeathFunction`
  (set `self.death` true)
  ;[1 1 1] Ölünce Healthbarı sil
  (bind _foundwidgets (`WidgetBlueprintLibrary.GetAllWidgetsOfClass` "/Game/Exol/UI/WBP_EnemyHealthBar.WBP_EnemyHealthBar_C"))
  (`Widget.RemoveFromParent` _foundwidgets)
  (`self.StopAnimMontage` null)
  (`BlackboardComponent.SetValueAsBool` (`AIBlueprintHelperLibrary.GetBlackboard` null) (`KismetStringLibrary.Conv_StringToName` "dead") true)
  (bind _asenemy_aicontroller (cast `/Game/Exol/AI/EnemyAIController` (`self.GetController`)))
  (`AIController.K2_ClearFocus` _asenemy_aicontroller)
  (`PrimitiveComponent.SetCollisionEnabled` (`self.CapsuleComponent`) "NoCollision")
  (`GameplayStatics.PlaySoundAtLocation` "/Game/Exol/Assets/Sound/SFX/E_Death.E_Death" (0.0 0.0 0.0) (struct) 1.0 1.0 0.0 null null null null)
  (set `self.SmoothRotation` false)
  ;[1 1 1] Send Enemy Dead Info and Save
  (bind _asbp_third_person_game_mode (cast `/Game/Unreal/ThirdPerson/Blueprints/BP_ThirdPersonGameMode` (`GameplayStatics.GetGameMode`)))
  (`/Game/Unreal/ThirdPerson/Blueprints/BP_ThirdPersonGameMode.EnemyDied` _asbp_third_person_game_mode (`self.IDEnemySave`))
  (bind _foundwidgets_2 (`WidgetBlueprintLibrary.GetAllWidgetsOfClass` "/Game/Exol/UI/WBP_Hit.WBP_Hit_C"))
  (for _array_element _foundwidgets_2
    (`Widget.RemoveFromParent` _array_element)))

(fn `EnemyHealthBarGenerator`
  ;[1 1 1] health bar create
  (bind _foundwidgets (`WidgetBlueprintLibrary.GetAllWidgetsOfClass` "/Game/Exol/UI/WBP_EnemyHealthBar.WBP_EnemyHealthBar_C"))
  (`Widget.RemoveFromParent` _foundwidgets)
  (bind _returnvalue (`|CreateWidget` "/Game/Exol/UI/WBP_EnemyHealthBar.WBP_EnemyHealthBar_C"))
  (set `self.WBP_EnemeyHealthBar` _returnvalue)
  (set `/Game/Exol/UI/WBP_EnemyHealthBar.WBP_Health` (`self.Health`) _returnvalue)
  (set `/Game/Exol/UI/WBP_EnemyHealthBar.WBP_MaxHealth` (`self.maxHealth`) _returnvalue))

(fn `Face Player`
  (bind (_returnvalue_roll _returnvalue_pitch _returnvalue_yaw) (`KismetMathLibrary.BreakRotator` (`KismetMathLibrary.RInterpTo` (`self.K2_GetActorRotation`) (`KismetMathLibrary.FindLookAtRotation` (`self.K2_GetActorLocation`) (`self.K2_GetActorLocation` (`GameplayStatics.GetPlayerPawn` 0))) (`GameplayStatics.GetWorldDeltaSeconds`) 7.0)))
  (if (`self.SmoothRotation`)
    (`self.K2_SetActorRotation` (`KismetMathLibrary.MakeRotator` 0.0 0.0 _returnvalue_yaw))))

(fn `HealthRegen`
  (locals (healthRegen :type "Float (double-precision)" :default 0.5))
  (if (< (`self.Health`) (`self.maxHealth`))
    (set `self.Health` (+ (`self.Health`) (* (`GameplayStatics.GetWorldDeltaSeconds`) (`local.healthRegen`))))))

(fn `IsParrySuccess`
  (returns (Success :type Boolean))
  (if (`self.CanParried`)
    (bind _asbp_player (cast `/Game/Exol/Blueprint/Bp_Player` (`GameplayStatics.GetPlayerPawn` 0)))
    (bind _returnvalue (== (`/Game/Exol/Blueprint/Bp_Player.Stance` _asbp_player) (`KismetMathLibrary.Conv_ByteToInt` (`self.PositionToGetParried`))))
    (if _returnvalue
      (return _returnvalue)
      (else
        (return _returnvalue)))
    (else
      (return false))))

(fn `Next Pos To Get Parried`
  (params (Direction :type "/Game/Exol/AI/BP_enum_direction Enum" :default "NewEnumerator0") (animation :type Boolean))
  (bind _foundwidgets (`WidgetBlueprintLibrary.GetAllWidgetsOfClass` "/Game/Exol/UI/WBP_Hit.WBP_Hit_C"))
  (if (> (`KismetArrayLibrary.Array_Length` _foundwidgets) 0)
    (for _array_element _foundwidgets
      (`Widget.RemoveFromParent` _array_element)))
  (switch `/Game/Exol/AI/BP_enum_direction` Direction
    (:`NewEnumerator1`
      (set `self.PositionToGetParried` "NewEnumerator2")
      (set `self.ParryScalarBPE` 0.125))
    (:`NewEnumerator2`
      (set `self.PositionToGetParried` "NewEnumerator1")
      (set `self.ParryScalarBPE` 0.375))
    (:`NewEnumerator3`
      (set `self.PositionToGetParried` "NewEnumerator4")
      (set `self.ParryScalarBPE` 0.625))
    (:`NewEnumerator4`
      (set `self.PositionToGetParried` "NewEnumerator3")
      (set `self.ParryScalarBPE` 0.875))
    (:`NewEnumerator5`
      (set `self.PositionToGetParried` "NewEnumerator5")
      (set `self.ParryScalarBPE` 0.25))
    (:`NewEnumerator6`
      (set `self.PositionToGetParried` "NewEnumerator6")
      (set `self.ParryScalarBPE` 0.75)))
  (bind _asbp_player (cast `/Game/Exol/Blueprint/Bp_Player` (`GameplayStatics.GetPlayerPawn` 0)))
  (bind _returnvalue (`|CreateWidget` "/Game/Exol/UI/WBP_Hit.WBP_Hit_C" (`GameplayStatics.GetPlayerController` 0) (`GameplayStatics.GetPlayerPawn` 0) (0.0 0.0 0.0) (`self.ParryScalarBPE`)))
  (set `self.HitIndicator` _returnvalue)
  (if animation
    (`/Game/Exol/UI/WBP_Hit.animasyon` _returnvalue))
  (if (`/Game/Exol/Blueprint/Bp_Player.isAttackUIOpen` _asbp_player)
    (if (== (`/Game/Exol/Blueprint/Bp_Player.TargetedEnemy` _asbp_player) self)
      (`UserWidget.AddToViewport` _returnvalue 0))))

(fn `NextPatrol`
  (`/Engine/EditorBlueprintResources/StandardMacros.IncrementInt` (`self.CurrentRoute`)))

(fn `PatrolLocation`
  (returns (PatrolLocation :type "Vector Structure"))
  (locals (TotalPoint :type Integer))
  (bind _spline (`/Game/Exol/AI/PatrolSpline.Spline` (`self.PatrolRoute`)))
  (bind _output_get (set `local.TotalPoint` (`SplineComponent.GetNumberOfSplinePoints` _spline)))
  (if (< _output_get (`self.CurrentRoute`))
    (set `self.CurrentRoute` 0))
  (return (`SplineComponent.GetLocationAtSplinePoint` _spline (`self.CurrentRoute`) "World")))

(fn `PAttackType`
  (returns (SpecialAttack :type Boolean))
  (bind _asbp_player (cast `/Game/Exol/Blueprint/Bp_Player` (`GameplayStatics.GetPlayerPawn` 0)))
  (bind _output_get (set `self.PlayerStance` (`/Game/Exol/Blueprint/Bp_Player.Stance` _asbp_player)))
  (switch `/Game/Exol/AI/BP_enum_direction` _output_get
    (:`NewEnumerator0`
      _)
    (:`NewEnumerator1`
      _)
    (:`NewEnumerator2`
      _)
    (:`NewEnumerator3`
      _)
    (:`NewEnumerator4`
      _)
    (:`NewEnumerator5`
      _)
    (:`NewEnumerator6`
      _)
    (:`NewEnumerator7`
      (set `self.PlayerDamage` 65.0)
      (`/Engine/EditorBlueprintResources/StandardMacros.DecrementFloat` (`self.Stamina`)
        (:`  `
          (set `self.PSpecial` true :!label _label)
          (return true))))
    (:`NewEnumerator8`
      (set `self.PlayerDamage` 80.0)
      (goto _label)))
  (set `self.PlayerDamage` 40.0)
  (set `self.PSpecial` false)
  (return false))

(fn `ShowIndicator`
  (bind _hitindicator (`self.HitIndicator`))
  (`/Engine/EditorBlueprintResources/StandardMacros.IsValid` _hitindicator
    (:`Is Valid`
      (`/Engine/EditorBlueprintResources/StandardMacros.IsValid` (`self.WBP_EnemeyHealthBar`)
        (:`Is Valid`
          (`UserWidget.AddToViewport` _hitindicator 0)
          (`UserWidget.AddToViewport` (`self.WBP_EnemeyHealthBar`) 0))))))

(fn `StaminaRegen`
  (locals (stRegen :type "Float (double-precision)" :default 0.1) (maxStamina :type "Float (double-precision)" :default 3.0))
  (if (< (`self.Stamina`) (`local.maxStamina`))
    (set `self.Stamina` (+ (`self.Stamina`) (* (`GameplayStatics.GetWorldDeltaSeconds`) (`local.stRegen`))))))

(fn `TakeDamage`
  (returns (Alive :type Boolean))
  (bind _wbp_enemeyhealthbar (`self.WBP_EnemeyHealthBar`))
  (set `self.CanParried` false)
  (if (> (`self.Health`) 0.0)
    (`AISense_Damage.ReportDamageEvent` self (`GameplayStatics.GetPlayerController` 0))
    (bind _output_get (set `self.Health` (- (`self.Health`) (`self.PlayerDamage`))))
    (`MovementComponent.StopMovementImmediately` (`self.CharacterMovement`))
    ;[1 1 1] Update Enemy Health Bar
    (set `/Game/Exol/UI/WBP_EnemyHealthBar.WBP_Health` _output_get _wbp_enemeyhealthbar)
    (set `/Game/Exol/UI/WBP_EnemyHealthBar.WBP_MaxHealth` (`self.maxHealth`) _wbp_enemeyhealthbar)
    (if (<= (`self.Health`) 0.0)
      (`self.DeathFunction`)
      (return false)
      (else
        (return true)))
    (else
      (return false))))

(fn `UserConstructionScript`
  (set `self.maxHealth` (`self.Health`))
  (if (`KismetStringLibrary.EqualEqual_StrStr` (`self.IDEnemySave`))
    (set `self.IDEnemySave` (`KismetGuidLibrary.Conv_GuidToString` (`KismetGuidLibrary.NewGuid`)))))