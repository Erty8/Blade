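; Level transition trigger that moves the game to the map named in LevelName when its box is overlapped.
; It shows a loading screen widget, then passes current health, stamina and the target map name to the game instance's save message.
; It stream-loads the level, waits briefly, then opens it by name.
; The overlapping actor is not filtered, and save-slot checks, deletion and interface-based stat saving are disconnected.
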(event `self.Box.OnComponentBeginOverlap`
  (params (OverlappedComponent :type "PrimitiveComponent Object Reference") (OtherActor :type "Actor Object Reference") (OtherComp :type "PrimitiveComponent Object Reference") (OtherBodyIndex :type Integer) (bFromSweep :type Boolean) (SweepResult :type "HitResult Structure (by ref)"))
  (bind _returnvalue (`GameplayStatics.GetGameInstance`))
  (bind _level_name (`self.Level Name`))
  (bind _returnvalue_2 (`|CreateWidget` "/Game/Exol/UI/Loading_Screen/WBP_LoadingScreen.WBP_LoadingScreen_C"))
  (`UserWidget.AddToViewport` _returnvalue_2 0)
  (bind _savegamedata (message `/Game/Exol/Blueprint/SaveSystem/BPI_SaveGame.GetGameData` _returnvalue))
  (bind (_playersave_playerhealth _playersave_playermaxhealth _playersave_playerstamina _playersave_playermaxstamina) (break `/Game/Exol/Blueprint/SaveSystem/S_PlayerSave` (`/Game/Exol/Blueprint/SaveSystem/BP_SaveGame.PlayerSave` _savegamedata)))
  (message `/Game/Exol/Blueprint/SaveSystem/BPI_SaveGame.SavePlayer` _returnvalue (make `/Game/Exol/Blueprint/SaveSystem/S_PlayerSave` _playersave_playerhealth _playersave_playermaxhealth _playersave_playerstamina _playersave_playermaxstamina "0.000000,0.000000,0.000000|0.000000,0.000000,0.000000|1.000000,1.000000,1.000000" (`KismetStringLibrary.Conv_NameToString` (`self.Level Name`))) false)
  (`GameplayStatics.LoadStreamLevel` _level_name true)
  (`KismetSystemLibrary.Delay` 1.0)
  (`GameplayStatics.OpenLevel` _level_name))

(fn `UserConstructionScript`)