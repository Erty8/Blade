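; Game instance that owns the save system, loading or creating a BP_SaveGame on Init and exposing it as SaveData.
; Loads and saves run sync or async, with OnGameLoaded fired after async loads and a saving widget created on saves.
; Player data and dead BP_Enemy object names are written into SaveData, saving once per killed name for enemies.
; DestroyKilledEnemies removes enemies whose names are saved, and DeleteSaveGame clears the slot.
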(event `self.ReceiveInit`
  (`self.LoadGameData` false))

(event `/Game/Exol/Blueprint/SaveSystem/BPI_SaveGame.LoadGameData`
  (params (Async :type Boolean))
  (bind _slotname (`self.SlotName`))
  ;[1 1 1] Load Game
  (bind _returnvalue (`GameplayStatics.DoesSaveGameExist` (`self.SlotName`)))
  (if _returnvalue
    (`KismetSystemLibrary.PrintString` "true")
    (if Async
      (bind _savegame (`AsyncActionHandleSaveGame.AsyncLoadGameFromSlot` _slotname)
        (:`Completed`
          (bind _asbp_save_game (cast `/Game/Exol/Blueprint/SaveSystem/BP_SaveGame` _savegame)
            (:`then`
              (set `self.SaveData` _asbp_save_game)
              ;;[1 1 1] Async Loada bindlanmak istenen başka bir event olursa diye bu OnGameLoaded event dispatcher eklendi
              (`self.OnGameLoaded`)
              (`KismetSystemLibrary.PrintString` "load game async"))
            (:`CastFailed`
              (`KismetSystemLibrary.PrintString` "cast faşked" :!label _label)))))
      (else
        (bind _returnvalue_2 (`GameplayStatics.LoadGameFromSlot` _slotname))
        (bind _asbp_save_game_2 (cast `/Game/Exol/Blueprint/SaveSystem/BP_SaveGame` _returnvalue_2)
          (:`then`
            (bind _output_get (set `self.SaveData` _asbp_save_game_2))
            (`KismetSystemLibrary.PrintString` "load game from save")
            (for _array_element (`/Game/Exol/Blueprint/SaveSystem/BP_SaveGame.killedEnemies` _output_get)
              (`KismetSystemLibrary.PrintString` _array_element true true (struct :`R` 1.0 :`G` 0.014757 :`A` 1.0))))
          (:`CastFailed`
            (goto _label)))))
    (else
      (`KismetSystemLibrary.PrintString` "false")
      (bind _returnvalue_3 (`GameplayStatics.CreateSaveGameObject` "/Game/Exol/Blueprint/SaveSystem/BP_SaveGame.BP_SaveGame_C"))
      (set `self.SaveData` _returnvalue_3)
      (`KismetSystemLibrary.PrintString` "created save"))))

(event `/Game/Exol/Blueprint/SaveSystem/BPI_SaveGame.SaveGameData`
  (params (Async :type Boolean))
  ;[1 1 1] SaveGame
  (if Async
    (`AsyncActionHandleSaveGame.AsyncSaveGameToSlot` (`self.SaveData`) (`self.SlotName`)
      (:`then`
        (`/Engine/EditorBlueprintResources/StandardMacros.IsValid` (`self.wbpSave`)
          (:`Is Not Valid`
            ;[1 1 1] Saving Widget - Flipbook olan
            (bind _returnvalue (`|CreateWidget` "/Game/Exol/UI/Loading_Screen/WBP_SavingFlip.WBP_SavingFlip_C"))
            (bind _output_get (set `self.wbpSave` _returnvalue))
            (`UserWidget.AddToViewport` _output_get 0)
            (`Widget.RemoveFromParent` (stale _output_get_2))))))
    (else
      (`GameplayStatics.SaveGameToSlot` (`self.SaveData`) (`self.SlotName`))
      (`/Engine/EditorBlueprintResources/StandardMacros.IsValid` (`self.wbpSave`)
        (:`Is Not Valid`
          (bind _returnvalue_2 (`|CreateWidget` "/Game/Exol/UI/Loading_Screen/WBP_SavingFlip.WBP_SavingFlip_C"))
          (bind _output_get_2 (set `self.wbpSave` _returnvalue_2))
          (`UserWidget.AddToViewport` _output_get_2 0)
          (`KismetSystemLibrary.Delay` 3.0)
          (`Widget.RemoveFromParent` _output_get_2)))))
  (set `self.wbpSave` null))

(event `/Game/Exol/Blueprint/SaveSystem/BPI_SaveGame.SavePlayer`
  (params (PlayerSave :type "/Game/Exol/Blueprint/SaveSystem/S_PlayerSave Structure") (Async :type Boolean))
  ;[1 1 1] SavePlayer
  (set `/Game/Exol/Blueprint/SaveSystem/BP_SaveGame.PlayerSave` PlayerSave (`self.SaveData`))
  (`self.SaveGameData` Async))

(event `/Game/Exol/Blueprint/SaveSystem/BPI_SaveGame.SaveKilledEnemies`
  (params (Async :type Boolean))
  (bind _killedenemies (`self.killedEnemies`))
  ;[1 1 1] SaveKilledEnemies
  (bind _outactors (`GameplayStatics.GetAllActorsOfClass` "/Game/Exol/Blueprint/Enemies/BP_Enemy.BP_Enemy_C"))
  (for _array_element _outactors
    (if (`/Game/Exol/Blueprint/Enemies/BP_Enemy.death` _array_element)
      (`KismetArrayLibrary.Array_AddUnique` _killedenemies (`KismetSystemLibrary.GetObjectName` _array_element))))
  (bind _output_get (set `/Game/Exol/Blueprint/SaveSystem/BP_SaveGame.killedEnemies` _killedenemies (`self.SaveData`)))
  (for _array_element_2 _output_get
    (`self.SaveGameData` Async))
  (for _ (`self.killedEnemies`)
    (`KismetSystemLibrary.PrintString` "ÖLÜ1")))

(event `/Game/Exol/Blueprint/SaveSystem/BPI_SaveGame.DestroyKilledEnemies`
  ;[1 1 1] Destroy Killed Enemies - suggested to call on level blueprint
  (bind _outactors (`GameplayStatics.GetAllActorsOfClass` "/Game/Exol/Blueprint/Enemies/BP_Enemy.BP_Enemy_C"))
  (for _array_element _outactors
    (if (`KismetArrayLibrary.Array_Contains` (`/Game/Exol/Blueprint/SaveSystem/BP_SaveGame.killedEnemies` (`self.SaveData`)) (`KismetSystemLibrary.GetObjectName` _array_element))
      (`Actor.K2_DestroyActor` _array_element)))
  (`KismetSystemLibrary.PrintString` "previously killed  enemies destroyed"))

(event `/Game/Exol/Blueprint/SaveSystem/BPI_SaveGame.DeleteSaveGame`
  ;[1 1 1] DeleteGameInSlot
  (`GameplayStatics.DeleteGameInSlot` (`self.SlotName`)))

(fn `GetGameData`
  (returns (SaveGameData :type "/Game/Exol/Blueprint/SaveSystem/BP_SaveGame Object Reference"))
  (return (`self.SaveData`)))