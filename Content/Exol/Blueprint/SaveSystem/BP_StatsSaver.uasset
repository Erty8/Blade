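; BP_StatsSaver is a one-shot checkpoint trigger that saves the player's stats, without location according to its debug message.
; When the player pawn overlaps its Box, a DoOnce gate calls SaveStats and prints that debug message.
; It then shows the WBP_CheckpointPassed widget briefly before removing it.
; GetID returns an empty string.
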(event `self.Box.OnComponentBeginOverlap`
  (params (OverlappedComponent :type "PrimitiveComponent Object Reference") (OtherActor :type "Actor Object Reference") (OtherComp :type "PrimitiveComponent Object Reference") (OtherBodyIndex :type Integer) (bFromSweep :type Boolean) (SweepResult :type "HitResult Structure (by ref)"))
  (if (== (`GameplayStatics.GetPlayerPawn` 0) OtherActor)
    (`/Engine/EditorBlueprintResources/StandardMacros.DoOnce` false
      (:`Completed`
        (`/Game/Exol/Blueprint/SaveSystem/BPI_SaveStats.SaveStats`)
        (`KismetSystemLibrary.PrintString` "savedOnlyPlayerStatsNOTLocation")
        (bind _returnvalue (`|CreateWidget` "/Game/Exol/Blueprint/SaveSystem/WBP_CheckpointPassed.WBP_CheckpointPassed_C"))
        (`UserWidget.AddToViewport` _returnvalue 0)
        (`KismetSystemLibrary.Delay` 2.0)
        (`Widget.RemoveFromParent` _returnvalue)))))

(fn `GetID`
  (returns (ID :type String))
  (return ""))

(fn `UserConstructionScript`)