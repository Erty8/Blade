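; Game instance that holds the game options and persists them through save game objects.
; Options are updated in memory, written to a dedicated slot as SG_Options, and loaded back, falling back to class defaults when no save exists.
; SaveStats is empty; the code that saves player health and stamina to SG_Stats is disconnected and never runs.
; GetID is a stub returning an empty string.
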(event `UpdateGameOptions`
  (params (Options :type "/Game/Exol/Blueprint/SaveSystem/OptionsStructure Structure"))
  (set `self.GameOptions` Options))

(event `SaveOptions`
  (bind _returnvalue (`GameplayStatics.CreateSaveGameObject` "/Game/Exol/Blueprint/SaveSystem/SG_Options.SG_Options_C"))
  (set `/Game/Exol/Blueprint/SaveSystem/SG_Options.Options` (`self.GameOptions`) _returnvalue)
  (`GameplayStatics.SaveGameToSlot` _returnvalue "OptionsSlot"))

(event `LoadOptions`
  (bind _returnvalue (`GameplayStatics.DoesSaveGameExist` "OptionsSlot"))
  (if _returnvalue
    (bind _returnvalue_2 (`GameplayStatics.LoadGameFromSlot` "OptionsSlot"))
    (bind _assg_options (cast `/Game/Exol/Blueprint/SaveSystem/SG_Options` _returnvalue_2))
    (set `self.GameOptions` (`/Game/Exol/Blueprint/SaveSystem/SG_Options.Options` _assg_options))
    (else
      (bind _returnvalue_3 (`GameplayStatics.CreateSaveGameObject` "/Game/Exol/Blueprint/SaveSystem/SG_Options.SG_Options_C"))
      (set `self.GameOptions` (`/Game/Exol/Blueprint/SaveSystem/SG_Options.Options` _returnvalue_3)))))

(event `SaveStats`)

(fn `GetID`
  (returns (ID :type String))
  (return ""))