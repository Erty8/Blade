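; AI-controlled melee enemy with directional attacks, parrying, blocking, stamina regeneration and death.
; Attack reads the blackboard Stance to pick a montage, shows a hit widget and opens a timed parry window.
; Player sword overlaps on the capsule apply damage, which triggers a counterattack if blocking, otherwise a parry check against player stance.
; Failed checks cost health and rebuild the health bar widget; death sets the blackboard flag and clears AI focus.
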(event `self.ReceiveTick`
  (params (DeltaSeconds :type "Float (single-precision)"))
  (`self.StaminaRegen`))

(event `self.Sphere.OnComponentBeginOverlap`
  (params (OverlappedComponent :type "PrimitiveComponent Object Reference") (OtherActor :type "Actor Object Reference") (OtherComp :type "PrimitiveComponent Object Reference") (OtherBodyIndex :type Integer) (bFromSweep :type Boolean) (SweepResult :type "HitResult Structure (by ref)"))
  (cast `/Game/Exol/Blueprint/Bp_Player` OtherActor)
  (set `self.playerInrange` true))

(event `self.Sphere.OnComponentEndOverlap`
  (params (OverlappedComponent :type "PrimitiveComponent Object Reference") (OtherActor :type "Actor Object Reference") (OtherComp :type "PrimitiveComponent Object Reference") (OtherBodyIndex :type Integer))
  (cast `/Game/Exol/Blueprint/Bp_Player` OtherActor)
  (set `self.playerInrange` false))

(event `self.ReceiveAnyDamage`
  (params (Damage :type "Float (single-precision)") (DamageType :type "DamageType Object Reference") (InstigatedBy :type "Controller Object Reference") (DamageCauser :type "Actor Object Reference"))
  (`self.CheckDamage`))

(event `Attack`
  ;[1 1 1] Attacking
  (set `self.Busy` true)
  (`self.Parriable`)
  (`self.PositionMacro`))

(event `Defend`
  (set `self.Busy` true)
  (set `self.Blocking` true)
  (`|PlayMontage` (`self.Mesh`) "/Game/Exol/Asset/Enemies/02/animations/BlockM.BlockM" 1.2
    (:`OnCompleted`
      (set `self.Blocking` false)
      (set `self.Busy` false))))

(event `Walk`
  (set `CharacterMovementComponent.MaxWalkSpeed` 150.0 (`self.CharacterMovement`)))

(event `Run`
  (set `CharacterMovementComponent.MaxWalkSpeed` 350.0 (`self.CharacterMovement`)))

(event `CounterAttack`
  (`KismetSystemLibrary.PrintString` "Counter Attack")
  (`KismetSystemLibrary.Delay` 0.0)
  (set `self.Blocking` false)
  (set `self.Busy` true)
  (`self.Attack`))

(event `Parriable`
  ;[0.2812 0.2812 0.2812] Parry
  (`self.GetParriedPosition`)
  (set `self.CanParried` true)
  (`KismetSystemLibrary.Delay` 1.2)
  (set `self.CanParried` false))

(event `CheckParry`
  ;[0.2812 0.2812 0.2812] Parry
  (bind _success (`self.IsParrySuccess`))
  (if _success
    (set `self.CanParried` false)
    (`|PlayMontage` (`self.Mesh`) "/Game/Exol/Asset/Enemies/02/animations/GetParried.GetParried" 0.8
      (:`OnCompleted`
        (set `self.Busy` false)))
    (else
      (`self.TakeDamage`)
      (`GameplayStatics.SpawnEmitterAtLocation` "/Game/StarterContent/Particles/P_Explosion.P_Explosion" (`self.K2_GetActorLocation`) (struct) (1.0 1.0 1.0) false))))

(event `self.CapsuleComponent.OnComponentBeginOverlap`
  (params (OverlappedComponent :type "PrimitiveComponent Object Reference") (OtherActor :type "Actor Object Reference") (OtherComp :type "PrimitiveComponent Object Reference") (OtherBodyIndex :type Integer) (bFromSweep :type Boolean) (SweepResult :type "HitResult Structure (by ref)"))
  ;[1 1 1] New combat system (collision based)
  (bind _asbp_player (cast `/Game/Exol/Blueprint/Bp_Player` OtherActor))
  (if (== OtherComp (`/Game/Exol/Blueprint/Bp_Player.SwordCol` _asbp_player))
    (if (`/Game/Exol/Blueprint/Bp_Player.SwordCollision` _asbp_player)
      (`GameplayStatics.ApplyDamage` self 40.0)
      (bind _output_get (set `self.Hit location` (`.ImpactPoint` (`GameplayStatics.BreakHitResult` SweepResult))))
      (`KismetSystemLibrary.PrintString` (`KismetStringLibrary.Conv_VectorToString` _output_get) true true (struct :`R` 1.0 :`G` 0.138097 :`A` 1.0) 5.0))))

(fn `CheckDamage`
  (if (`self.Blocking`)
    (`KismetSystemLibrary.PrintString` "blocked")
    (set `self.Stamina` (`KismetMathLibrary.Conv_IntToDouble` (- (`self.Stamina`) 1)))
    (`self.CounterAttack`)
    (else
      (`self.CheckParry`))))

(fn `GetParriedPosition`
  (switch `/Game/Exol/UI/BP_enum_direction` (cast `/Game/Exol/UI/BP_enum_direction` (`BlackboardComponent.GetValueAsEnum` (`AIBlueprintHelperLibrary.GetBlackboard` null) (`KismetStringLibrary.Conv_StringToName` "Stance")))
    (:`NewEnumerator1`
      (set `self.PositionToGetParried` "NewEnumerator2")
      (set `self.ParryScalarBPE` 0.125))
    (:`NewEnumerator2`
      (set `self.PositionToGetParried` "NewEnumerator1")
      (set `self.ParryScalarBPE` 0.375))
    (:`NewEnumerator3`
      (set `self.PositionToGetParried` "NewEnumerator4")
      (set `self.ParryScalarBPE` 0.625))
    (:`NewEnumerator4`
      (set `self.PositionToGetParried` "NewEnumerator3")
      (set `self.ParryScalarBPE` 0.875)))
  (bind _returnvalue (`|CreateWidget` "/Game/Exol/UI/WBP_Hit.WBP_Hit_C" (`GameplayStatics.GetPlayerController` 0) (`GameplayStatics.GetPlayerPawn` 0) (0.0 0.0 0.0) (`self.ParryScalarBPE`)))
  (`UserWidget.AddToViewport` _returnvalue 0))

(fn `HealthRegen`
  (locals (healthRegen :type "Float (double-precision)" :default 0.5))
  (if (< (`self.Health`) (`self.maxHealth`))
    (set `self.Health` (+ (`self.Health`) (* (`GameplayStatics.GetWorldDeltaSeconds`) (`local.healthRegen`))))))

(fn `IsParrySuccess`
  (returns (Success :type Boolean))
  (if (`self.CanParried`)
    (bind _asbp_player (cast `/Game/Exol/Blueprint/Bp_Player` (`GameplayStatics.GetPlayerPawn` 0)))
    (bind _returnvalue (== (`/Game/Exol/Blueprint/Bp_Player.Stance` _asbp_player) (`KismetMathLibrary.Conv_ByteToInt` (`self.PositionToGetParried`))))
    (if _returnvalue
      (return _returnvalue)
      (else
        (return _returnvalue)))
    (else
      (`KismetSystemLibrary.PrintString` "out of parry window")
      (return false))))

(fn `StaminaRegen`
  (locals (stRegen :type "Float (double-precision)" :default 0.1) (maxStamina :type "Float (double-precision)" :default 3.0))
  (if (< (`self.Stamina`) (`local.maxStamina`))
    (set `self.Stamina` (+ (`self.Stamina`) (* (`GameplayStatics.GetWorldDeltaSeconds`) (`local.stRegen`))))))

(fn `TakeDamage`
  (bind _output_get (set `self.Health` (- (`self.Health`) 40.0)))
  ;[1 1 1] Create HealthBar Enemy Widget
  (bind _foundwidgets (`WidgetBlueprintLibrary.GetAllWidgetsOfClass` "/Game/Exol/UI/WBP_EnemyHealthBar.WBP_EnemyHealthBar_C"))
  (`Widget.RemoveFromParent` _foundwidgets)
  (bind _returnvalue (`|CreateWidget` "/Game/Exol/UI/WBP_EnemyHealthBar.WBP_EnemyHealthBar_C"))
  (bind _output_get_2 (set `self.WBP_EnemeyHealthBar` _returnvalue))
  (set `/Game/Exol/UI/WBP_EnemyHealthBar.WBP_Health` _output_get _output_get_2)
  (set `/Game/Exol/UI/WBP_EnemyHealthBar.WBP_MaxHealth` (`self.maxHealth`) _output_get_2)
  (`UserWidget.AddToViewport` _output_get_2 0)
  (`KismetSystemLibrary.PrintString` (`KismetStringLibrary.Conv_DoubleToString` _output_get))
  (`KismetSystemLibrary.PrintString` "Enemy Health")
  (if (<= (`self.Health`) 0.0)
    (set `self.death` true)
    ;[1 1 1] Ölünce Healthbarı sil
    (bind _foundwidgets_2 (`WidgetBlueprintLibrary.GetAllWidgetsOfClass` "/Game/Exol/UI/WBP_EnemyHealthBar.WBP_EnemyHealthBar_C"))
    (`Widget.RemoveFromParent` _foundwidgets_2)
    (`self.StopAnimMontage` null)
    (`BlackboardComponent.SetValueAsBool` (`AIBlueprintHelperLibrary.GetBlackboard` null) (`KismetStringLibrary.Conv_StringToName` "dead") true)
    (bind _asenemy_aicontroller (cast `/Game/Exol/AI/EnemyAIController` (`self.GetController`)))
    (`AIController.K2_ClearFocus` _asenemy_aicontroller)))

(fn `UserConstructionScript`
  (set `self.Health` 100.0))