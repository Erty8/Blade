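; BP_ItemSword is a collectible sword that shows its widget while something overlaps its trigger.
; PickUpInteract unhides the player, plays the sword-take montage, destroys actors tagged "warpSword", calls DestroyItem and returns the sword's static mesh.
; DestroyItem hides the widget and fades out audio, then uses delays to hide the mesh mid-fade and destroy the actor once the fade has finished.
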(event `DestroyItem`
  (`SceneComponent.SetVisibility` (`self.Widget`) false false)
  (`AudioComponent.FadeOut` (`self.Audio`) 9.0 0.0 "Linear")
  (`KismetSystemLibrary.Delay` 2.0)
  (`SceneComponent.SetVisibility` (`self.StaticMesh`) false false)
  (`KismetSystemLibrary.Delay` 8.0)
  (`self.K2_DestroyActor`))

(event `self.Trigger.OnComponentBeginOverlap`
  (params (OverlappedComponent :type "PrimitiveComponent Object Reference") (OtherActor :type "Actor Object Reference") (OtherComp :type "PrimitiveComponent Object Reference") (OtherBodyIndex :type Integer) (bFromSweep :type Boolean) (SweepResult :type "HitResult Structure (by ref)"))
  (`SceneComponent.SetVisibility` (`self.Widget`) true false))

(event `self.Trigger.OnComponentEndOverlap`
  (params (OverlappedComponent :type "PrimitiveComponent Object Reference") (OtherActor :type "Actor Object Reference") (OtherComp :type "PrimitiveComponent Object Reference") (OtherBodyIndex :type Integer))
  (`SceneComponent.SetVisibility` (`self.Widget`) false false))

(fn `PickUpInteract`
  (returns (StaticMesh :type "StaticMesh Object Reference"))
  (bind _asbp_player (cast `/Game/Exol/Blueprint/Bp_Player` (`GameplayStatics.GetPlayerPawn` 0)))
  (`self.SetActorHiddenInGame` _asbp_player false)
  (set `/Game/Exol/Blueprint/Bp_Player.playerHidden` false _asbp_player)
  (`/Game/Exol/Blueprint/Bp_Player.SwordTakeMontage` _asbp_player)
  (bind _outactors (`GameplayStatics.GetAllActorsWithTag` "warpSword"))
  (`self.K2_DestroyActor` _outactors)
  (`self.DestroyItem`)
  (return (`StaticMeshComponent.StaticMesh` (`self.StaticMesh`))))

(fn `UserConstructionScript`)