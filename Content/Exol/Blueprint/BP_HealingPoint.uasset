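; BP_HealingPoint is a single-use healing pickup point that restores a Bp_Player to full health when they overlap its box.
; A DoOnce gates the overlap, which sets Health to MaxHealth and refreshes the HUD bar with hard-coded full values rather than the player's own.
; It then plays audio with a fade-out while a timeline animates the spotlight's intensity.
; The Interact event is empty, and an older heal path is left disconnected.
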(event `/Game/Exol/UI/Dialogue/BPI_Interact.Interact`)

(event `self.Box.OnComponentBeginOverlap`
  (params (OverlappedComponent :type "PrimitiveComponent Object Reference") (OtherActor :type "Actor Object Reference") (OtherComp :type "PrimitiveComponent Object Reference") (OtherBodyIndex :type Integer) (bFromSweep :type Boolean) (SweepResult :type "HitResult Structure (by ref)"))
  (bind _audio (`self.Audio`))
  (bind _asbp_player (cast `/Game/Exol/Blueprint/Bp_Player` OtherActor))
  (`/Engine/EditorBlueprintResources/StandardMacros.DoOnce` false
    (:`Completed`
      (set `/Game/Exol/Blueprint/Bp_Player.Health` (`/Game/Exol/Blueprint/Bp_Player.MaxHealth` _asbp_player) _asbp_player)
      (`/Game/Exol/UI/WBP_Hud.ClearHealthBar` (`/Game/Exol/Blueprint/Bp_Player.WBP_HUD_Variable` _asbp_player))
      (`/Game/Exol/UI/WBP_Hud.UpdateHealthBar` (`/Game/Exol/Blueprint/Bp_Player.WBP_HUD_Variable` _asbp_player) 100.0 100.0)
      (`AudioComponent.Play` _audio 0.0)
      (`AudioComponent.FadeOut` _audio 4.0 0.0 "Linear")
      (bind (_direction _newtrack_0) (`Timeline|Timeline`)
        (:`Update`
          (`LightComponent.SetIntensity` (`self.SpotLight`) _newtrack_0))))))

(fn `UserConstructionScript`)