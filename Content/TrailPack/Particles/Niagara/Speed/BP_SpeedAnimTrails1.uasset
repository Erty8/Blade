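; Timed Niagara anim notify state that drives a speed trail effect during an animation.
; Each tick it writes the mesh's Start and End socket locations into the spawned effect's StartTrail and EndTrail vector parameters.
; Updates run only while player 0's Bp_Player has Combo set, though a failed cast logs a message and still updates the trail.
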(fn `Received_NotifyTick`
  (params (MeshComp :type "SkeletalMeshComponent Object Reference") (Animation :type "AnimSequenceBase Object Reference") (FrameDeltaTime :type "Float (single-precision)") (EventReference :type "AnimNotifyEventReference Structure (by ref)"))
  (returns (ReturnValue :type Boolean))
  (bind _returnvalue (`self.GetSpawnedEffect` MeshComp))
  (`/Engine/EditorBlueprintResources/StandardMacros.IsValid` _returnvalue
    (:`Is Valid`
      (bind _asbp_player (cast `/Game/Exol/Blueprint/Bp_Player` (`GameplayStatics.GetPlayerPawn` MeshComp))
        (:`then`
          (if (`/Game/Exol/Blueprint/Bp_Player.Combo` _asbp_player)
            (`FXSystemComponent.SetVectorParameter` _returnvalue "StartTrail" (`SceneComponent.GetSocketLocation` MeshComp (`self.Start`)) :!label _label)
            (`FXSystemComponent.SetVectorParameter` _returnvalue "EndTrail" (`SceneComponent.GetSocketLocation` MeshComp (`self.End`)))
            (return false)))
        (:`CastFailed`
          (`KismetSystemLibrary.PrintString` null "cast failed")
          (goto _label))))
    (:`Is Not Valid`
      (`KismetSystemLibrary.PrintString` null "Trail Not Valid")
      (return false))))